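; BP_Pawn is a pawn that moves along a spline, with input to adjust or toggle its speed.
; Tick accumulates distance from Speed, sets the actor transform from the spline's local-space location and rotation, and resets distance past the end when looping.
; Input actions step Speed up or down by Increment, and a FlipFlop on Stop Pawn alternates between zero and a hard-coded speed.
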(event `self.ReceiveTick`
  (params (DeltaSeconds :type "Float (single-precision)"))
  (bind _spline (`self.Spline`))
  (bind _output_get (set `self.Distance` (+ (* DeltaSeconds (`self.speed`)) (`self.Distance`))))
  (bind (_returnvalue_location _returnvalue_rotation) (`KismetMathLibrary.BreakTransform` (`SplineComponent.GetTransformAtDistanceAlongSpline` _spline _output_get "Local" false)))
  (`self.K2_SetActorTransform` (`KismetMathLibrary.MakeTransform` _returnvalue_location _returnvalue_rotation))
  (if (`self.IsLooping`)
    (if (> (`self.Distance`) (`SplineComponent.GetSplineLength` _spline))
      (set `self.Distance` 0.0))))

(event `InputAction|Increase Speed`
  (params (Key :type "Key Structure"))
  ;[1 1 1] increase / decrease speed
  (:`Pressed`
    (set `self.speed` (+ (`self.increment`) (`self.speed`)))))

(event `InputAction|Decrease Speed`
  (params (Key :type "Key Structure"))
  ;[1 1 1] increase / decrease speed
  (:`Pressed`
    (set `self.speed` (- (`self.speed`) (`self.increment`)))))

(event `InputAction|Stop Pawn`
  (params (Key :type "Key Structure"))
  (:`Pressed`
    (`/Engine/EditorBlueprintResources/StandardMacros.FlipFlop`
      (:`A`
        (set `self.speed` 0.0))
      (:`B`
        (set `self.speed` 500.0)))))

(fn `UserConstructionScript`)